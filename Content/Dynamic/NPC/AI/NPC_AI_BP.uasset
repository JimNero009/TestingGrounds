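; NPC AI controller Blueprint that runs a guard behavior tree and reacts to perceived actors.
; On BeginPlay it sets up the PatrolData blackboard, starts GuardBehaviour and caches the blackboard component.
; AI perception updates write successfully sensed actors without the "Enemy" tag to the FocusPoint key.
; A failed sense of such an actor clears the key, while Enemy-tagged actors are ignored.
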(event `self.ReceiveBeginPlay`
  (bind _blackboardcomponent (`self.UseBlackboard` "/Game/Dynamic/NPC/AI/PatrolData.PatrolData"))
  (`self.RunBehaviorTree` "/Game/Dynamic/NPC/AI/GuardBehaviour.GuardBehaviour")
  (set `self.BlackboradComp` _blackboardcomponent))

(event `self.AIPerception.OnTargetPerceptionUpdated`
  (params (Actor :type "Actor Object Reference") (Stimulus :type "AIStimulus Structure"))
  (bind _returnvalue (`KismetStringLibrary.Conv_StringToName` "FocusPoint"))
  (if (`self.ActorHasTag` Actor "Enemy")
    _
    (elif (`.bSuccessfullySensed` (break `AIStimulus` Stimulus))
      (`BlackboardComponent.SetValueAsObject` (`self.BlackboradComp`) _returnvalue Actor)
      (else
        (`BlackboardComponent.ClearValue` (stale `self.ReceiveBeginPlay` _blackboardcomponent) _returnvalue)))))

(fn `UserConstructionScript`)