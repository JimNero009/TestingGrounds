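; NPC AI controller that drives guard behaviour through the GuardBehaviour tree and the PatrolData blackboard, both started on BeginPlay.
; AI Perception updates feed UpdateFocusPoint, which ignores invalid actors and those tagged Enemy.
; For other actors, a successful sense stores the actor in the FocusPoint blackboard key, and an unsuccessful one clears that key.
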(event `self.ReceiveBeginPlay`
  (bind _blackboardcomponent (`self.UseBlackboard` "/Game/Dynamic/Actor/AI/PatrolData.PatrolData"))
  (`self.RunBehaviorTree` "/Game/Dynamic/Actor/AI/GuardBehaviour.GuardBehaviour")
  (set `self.BlackboradComp` _blackboardcomponent))

(event `self.AIPerception.OnTargetPerceptionUpdated`
  (params (Actor :type "Actor Object Reference") (Stimulus :type "AIStimulus Structure"))
  (`self.UpdateFocusPoint` Actor Stimulus Actor))

(fn `UpdateFocusPoint`
  (params (ObjectValue :type "Object Object Reference") (AIStimulus :type "AIStimulus Structure (by ref)") (self2 :type "Actor Object Reference"))
  (bind _returnvalue (`KismetStringLibrary.Conv_StringToName` "FocusPoint"))
  (bind _blackboradcomp (`self.BlackboradComp`))
  (`/Engine/EditorBlueprintResources/StandardMacros.IsValid` self2
    (:`Is Valid`
      (if (`self.ActorHasTag` self2 "Enemy")
        _
        (elif (`.bSuccessfullySensed` (break `AIStimulus` AIStimulus))
          (`BlackboardComponent.SetValueAsObject` _blackboradcomp _returnvalue ObjectValue)
          (else
            (`BlackboardComponent.ClearValue` _blackboradcomp _returnvalue)))))))

(fn `UserConstructionScript`)