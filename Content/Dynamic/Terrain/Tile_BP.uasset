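; Terrain tile Blueprint with a barrier that lets the player through only while they overlap the tile's Box trigger.
; The barrier starts solid and red, and Box begin and end overlaps call Unlock and Lock.
; Both functions act only on player character 0, toggling the barrier's collision and swapping between red and green materials.
; GetAttachLocation exposes the AttachPoint world transform.
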(event `self.ReceiveBeginPlay`
  (bind _barrier (`self.Barrier`))
  (`PrimitiveComponent.SetCollisionEnabled` _barrier "QueryAndPhysics")
  (`PrimitiveComponent.SetMaterial` _barrier 0 "/Game/Dynamic/Terrain/RedBarrier.RedBarrier"))

(event `self.Box.OnComponentBeginOverlap`
  (params (OverlappedComponent :type "PrimitiveComponent Object Reference") (OtherActor :type "Actor Object Reference") (OtherComp :type "PrimitiveComponent Object Reference") (OtherBodyIndex :type Integer) (bFromSweep :type Boolean) (SweepResult :type "HitResult Structure (by ref)"))
  (`self.Unlock` OtherActor))

(event `self.Box.OnComponentEndOverlap`
  (params (OverlappedComponent :type "PrimitiveComponent Object Reference") (OtherActor :type "Actor Object Reference") (OtherComp :type "PrimitiveComponent Object Reference") (OtherBodyIndex :type Integer))
  (`self.Lock` OtherActor))

(fn `GetAttachLocation`
  (returns (AttachLocation :type "Transform Structure"))
  (return (`SceneComponent.K2_GetComponentToWorld` (`self.AttachPoint`))))

(fn `Lock`
  (params (PlayerRef :type "Actor Object Reference"))
  (bind _barrier (`self.Barrier`))
  (if (== PlayerRef (`GameplayStatics.GetPlayerCharacter` 0))
    (`PrimitiveComponent.SetCollisionEnabled` _barrier "QueryAndPhysics")
    (`PrimitiveComponent.SetMaterial` _barrier 0 "/Game/Dynamic/Terrain/RedBarrier.RedBarrier")))

(fn `Unlock`
  (params (PlayerREf :type "Actor Object Reference"))
  (if (== PlayerREf (`GameplayStatics.GetPlayerCharacter` 0))
    (`PrimitiveComponent.SetCollisionEnabled` (`self.Barrier`) "NoCollision")
    (`PrimitiveComponent.SetMaterial` (`self.Barrier`) 0 "/Game/Dynamic/Terrain/GreenBarrier.GreenBarrier")))

(fn `UserConstructionScript`)